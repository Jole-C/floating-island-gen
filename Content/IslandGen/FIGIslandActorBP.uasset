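; Procedural island actor that builds its mesh with Geometry Script when RegenerateIsland runs.
; GenerateCone unions inverted cones with level tops, each sized and offset from a randomly picked earlier cone after the first.
; Upward-facing polygroups get grass over dirt, then the mesh is remeshed, sine-warped, normal-repaired, scaled and randomly yawed.
; Collision is finally built as convex hulls; the iterative smoothing node is left unconnected.
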(event EventRegenerateIsland
  (Utilities|FlowControl|Sequence
    (:then_0
      ;[1 1 1] Set up materials
      (Class|DynamicMeshComponent|ConfigureMaterialSet (Variables|Default|GetDynamicMeshComponent) (Utilities|Array|MakeArray (Variables|Default|GetDirtMaterial) (Variables|Default|GetGrassMaterial))))
    (:then_1
      ;[1 1 1] Set up base mesh by appending and applying boolean to cones
      (bind _returnvalue (DynamicMeshComponent|GetDynamicMesh (Variables|Default|GetDynamicMeshComponent)))
      (Variables|Default|SetTargetMesh _returnvalue)
      (for _index (range 1 (Variables|/Script/FloatingIslandGen.IslandParameterDefinition|GetNumberOfCones (Variables|Default|GetIslandParameters)))
        (CallFunction|GenerateCone)))
    (:then_2
      ;[1 1 1] Apply material to poly groups based on normal dot product
      (bind _triangleidlist (GeometryScript|MeshQueries|GetAllTriangleIDs (Variables|Default|GetTargetMesh)))
      (bind _indexarray (Class|GeometryScriptLibraryListUtilityFunctions|ConvertIndexListtoArray _triangleidlist))
      (for _array_element _indexarray
        (if (> (Math|Vector|DotProduct (.ReturnValue (Class|GeometryScriptLibraryMeshQueryFunctions|GetTriangleFaceNormal (Variables|Default|GetTargetMesh) _array_element)) (Math|Vector|VectorUp)) 0.95)
          (Class|GeometryScriptLibraryMeshMaterialFunctions|SetPolygroupMaterialID :TargetMesh (Variables|Default|GetTargetMesh) :PolygroupID (.ReturnValue (Class|GeometryScriptLibraryMeshPolygroupFunctions|GetTrianglePolygroupID :TargetMesh (Variables|Default|GetTargetMesh) :TriangleID _array_element)) :MaterialID 1 :Debug 0))))
    (:then_3
      ;[1 1 1] Apply cleanup and various methods to mesh to improve appearence
      (bind _returnvalue_2 (Class|GeometryScriptLibraryRemeshingFunctions|ApplyUniformRemesh :TargetMesh (Variables|Default|GetTargetMesh) :UniformOptions (Utilities|Struct|MakeGeometryScriptUniformRemeshOptions "TriangleCount" (Variables|/Script/FloatingIslandGen.IslandParameterDefinition|GetRemeshTriangleCount (Variables|Default|GetIslandParameters)) 5e+01) :Debug 0))
      (bind _returnvalue_3 (Class|GeometryScriptLibraryMeshDeformFunctions|ApplyMathWarptoMesh :TargetMesh _returnvalue_2 :WarpType "SinWave2D" :Options (Utilities|Struct|MakeGeometryScriptMathWarpOptions (Variables|/Script/FloatingIslandGen.IslandParameterDefinition|GetWarpMagnitude (Variables|Default|GetIslandParameters)) (Variables|/Script/FloatingIslandGen.IslandParameterDefinition|GetWarpFrequency (Variables|Default|GetIslandParameters)) 0.0) :Debug 0))
      (bind _returnvalue_4 (GeometryScript|Normals|RecomputeNormals :TargetMesh _returnvalue_3 :bDeferChangeNotifications true :Debug 0))
      (bind _returnvalue_5 (Class|GeometryScriptLibraryMeshNormalsFunctions|AutoRepairNormals _returnvalue_4 0)))
    (:then_4
      ;[1 1 1] Set island scale
      (Class|GeometryScriptLibraryMeshTransformFunctions|ScaleMesh (Variables|Default|GetTargetMesh) (Variables|/Script/FloatingIslandGen.IslandParameterDefinition|GetIslandScale (Variables|Default|GetIslandParameters)) "0.000000,0.000000,0.000000" true 0))
    (:then_5
      ;[1 1 1] Set random rotation
      (Class|GeometryScriptLibraryMeshTransformFunctions|RotateMesh (Variables|Default|GetTargetMesh) (Math|Rotator|MakeRotator 0.0 0.0 (Math|Random|RandomFloatinRange 0.0 3.6e+02)) "0.000000,0.000000,0.000000" 0))
    (:then_6
      ;[1 1 1] Set up collision
      (Class|GeometryScriptLibraryCollisionFunctions|SetDynamicMeshCollisionfromMesh (Variables|Default|GetTargetMesh) (Variables|Default|GetDynamicMeshComponent) (Utilities|Struct|MakeGeometryScriptCollisionfromMeshOptions true "ConvexHulls" true true true 0.25) 0))))

(fn ConstructionScript)

(fn GenerateCone
  (bind _returnvalue (Math|Random|RandomFloatinRange 0.0 3.6e+02))
  (bind _generatedconeparameters (Variables|Default|GetGeneratedConeParameters))
  (bind (_outitem _outindex) (Utilities|Array|Random _generatedconeparameters))
  (Utilities|FlowControl|Sequence
    (:then_0
      ;[1 1 1] Depending on number of generated cones, set the selected cone to either the base cone parameters or a randomly chosen cone
      (if (== (Utilities|Array|Length (Variables|Default|GetGeneratedConeParameters)) 0)
        (LocalVariables|SetSelectedCone (Utilities|Struct|MakeConeParams (Variables|/Script/FloatingIslandGen.IslandParameterDefinition|GetBaseConeWidth (Variables|Default|GetIslandParameters)) (Variables|/Script/FloatingIslandGen.IslandParameterDefinition|GetBaseConeHeight (Variables|Default|GetIslandParameters)) "0.000000,0.000000,0.000000"))
        (Development|PrintString "Default cone selected")
        (else
          (LocalVariables|SetSelectedCone _outitem)
          (Development|PrintText (Utilities|Text|FormatText "cone {0} selected" _outindex))
          (LocalVariables|SetDontCentreCone true))))
    (:then_1
      ;[1 1 1] Calculate the cone's width and height based on the selected cone's width and height divided by the specified dividend, plus random deviation
      (Utilities|FlowControl|Sequence
        (:then_0
          (LocalVariables|SetConeWidth (Math|Float|Clamp(Float) (+ (/ (.ConeWidth (Utilities|Struct|BreakConeParams (LocalVariables|GetSelectedCone))) (Variables|/Script/FloatingIslandGen.IslandParameterDefinition|GetConeWidthDividend (Variables|Default|GetIslandParameters))) (Math|Random|RandomFloatinRange (* (Variables|/Script/FloatingIslandGen.IslandParameterDefinition|GetRandomWidthDeviation (Variables|Default|GetIslandParameters)) -1.0) (Variables|/Script/FloatingIslandGen.IslandParameterDefinition|GetRandomWidthDeviation (Variables|Default|GetIslandParameters)))) (Variables|/Script/FloatingIslandGen.IslandParameterDefinition|GetMinimumConeWidth (Variables|Default|GetIslandParameters)) (Variables|/Script/FloatingIslandGen.IslandParameterDefinition|GetBaseConeWidth (Variables|Default|GetIslandParameters)))))
        (:then_1
          (LocalVariables|SetConeHeight (Math|Float|Clamp(Float) (+ (/ (.ConeHeight (Utilities|Struct|BreakConeParams (LocalVariables|GetSelectedCone))) (Variables|/Script/FloatingIslandGen.IslandParameterDefinition|GetConeHeightDividend (Variables|Default|GetIslandParameters))) (Math|Random|RandomFloatinRange (* (Variables|/Script/FloatingIslandGen.IslandParameterDefinition|GetRandomHeightDeviation (Variables|Default|GetIslandParameters)) -1.0) (Variables|/Script/FloatingIslandGen.IslandParameterDefinition|GetRandomHeightDeviation (Variables|Default|GetIslandParameters)))) (Variables|/Script/FloatingIslandGen.IslandParameterDefinition|GetMinimumConeHeight (Variables|Default|GetIslandParameters)) (Variables|/Script/FloatingIslandGen.IslandParameterDefinition|GetBaseConeHeight (Variables|Default|GetIslandParameters)))))))
    (:then_2
      ;[1 1 1] Calculate the position from the selected cone's position plus a random angle, accounting for the base origin to ensure they're aligned vertically
      (LocalVariables|SetConePosition (+ (Math|Vector|SelectVector (Math|Vector|MakeVector (* (Math|Trig|Cos(Degrees) _returnvalue) (.ConeWidth (Utilities|Struct|BreakConeParams (LocalVariables|GetSelectedCone)))) (* (Math|Trig|Sin(Degrees) _returnvalue) (.ConeWidth (Utilities|Struct|BreakConeParams (LocalVariables|GetSelectedCone)))) (- (- (Variables|/Script/FloatingIslandGen.IslandParameterDefinition|GetBaseConeHeight (Variables|Default|GetIslandParameters)) (LocalVariables|GetConeHeight)) (Variables|/Script/FloatingIslandGen.IslandParameterDefinition|GetBaseConeHeight (Variables|Default|GetIslandParameters)))) (Math|Vector|MakeVector 0.0 0.0 (- (- (Variables|/Script/FloatingIslandGen.IslandParameterDefinition|GetBaseConeHeight (Variables|Default|GetIslandParameters)) (LocalVariables|GetConeHeight)) (Variables|/Script/FloatingIslandGen.IslandParameterDefinition|GetBaseConeHeight (Variables|Default|GetIslandParameters)))) (LocalVariables|GetDontCentreCone)) (Math|Vector|MakeVector (.X (Math|Vector|BreakVector (.ConePosition (Utilities|Struct|BreakConeParams (LocalVariables|GetSelectedCone))))) (.Y (Math|Vector|BreakVector (.ConePosition (Utilities|Struct|BreakConeParams (LocalVariables|GetSelectedCone))))) 0.0))))
    (:then_3
      ;[1 1 1] Using the calculated values, append a cone, then apply self union to it
      (bind _returnvalue_2 (Class|GeometryScriptLibraryMeshPrimitiveFunctions|AppendCone :TargetMesh (Variables|Default|GetTargetMesh) :Transform (Math|Transform|MakeTransform (LocalVariables|GetConePosition)) :BaseRadius (Variables|/Script/FloatingIslandGen.IslandParameterDefinition|GetIslandTipWidth (Variables|Default|GetIslandParameters)) :TopRadius (LocalVariables|GetConeWidth) :Height (LocalVariables|GetConeHeight) :RadialSteps 8 :HeightSteps 6 :Debug 0))
      (Class|GeometryScriptLibraryMeshBooleanFunctions|ApplyMeshSelfUnion :TargetMesh _returnvalue_2 :Debug 0)
      ;[1 1 1] Add a new cone to the array using the calculated values
      (Utilities|Array|Add (Variables|Default|GetGeneratedConeParameters) (Utilities|Struct|MakeConeParams (LocalVariables|GetConeWidth) (LocalVariables|GetConeHeight) (LocalVariables|GetConePosition))))))