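; Prop actor for island generation that shows a random static mesh at a random facing.
; SelectRandomMesh picks an entry from the Meshes array for the StaticMesh component and replaces the actor's rotation with a random yaw, zeroing pitch and roll.
; It runs in the construction script and again through the PickNewMesh event, using unseeded randomness, so each rerun can change the result.
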(event Custom|PickNewMesh
  (CallFunction|SelectRandomMesh))

(fn ConstructionScript
  (CallFunction|SelectRandomMesh))

(fn SelectRandomMesh
  (Components|StaticMesh|SetStaticMesh (Variables|Default|GetStaticMesh) (.OutItem (Utilities|Array|Random (Variables|Default|GetMeshes))))
  (Transformation|SetActorRotation (Math|Rotator|MakeRotator 0.0 0.0 (Math|Random|RandomFloatinRange 0.0 3.6e+02))))